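; Item pickup for vehicles that grants a random item when a VehicleBlueprint overlaps its collider while holding none.
; On pickup it sets one of three items on the vehicle, hides its mesh and blocks further pickups until a five-second timer respawns it.
; Tick spins the mesh and bobs it on a sine wave driven by time since creation.
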(event `self.Collider.OnComponentBeginOverlap`
  (params (OverlappedComponent :type "PrimitiveComponent Object Reference") (OtherActor :type "Actor Object Reference") (OtherComp :type "PrimitiveComponent Object Reference") (OtherBodyIndex :type Integer) (bFromSweep :type Boolean) (SweepResult :type "HitResult Structure (by ref)"))
  ;[1 1 1] Touched by a Car
  (if (not (`self.Respawning`))
    (bind _asvehicle_blueprint (cast `/Game/VehicleAdvBP/Blueprints/VehicleBlueprint` OtherActor))
    (switch `/Game/Items/UI/Item_ENUM` (`/Game/VehicleAdvBP/Blueprints/VehicleBlueprint.CurrentItem` _asvehicle_blueprint)
      (:`NewEnumerator0`
        (`/Game/VehicleAdvBP/Blueprints/VehicleBlueprint.SetItem` _asvehicle_blueprint (cast `/Game/Items/UI/Item_ENUM` (`KismetMathLibrary.Conv_IntToByte` (`KismetMathLibrary.RandomIntegerInRange` 1 3))))
        (set `/Game/VehicleAdvBP/Blueprints/VehicleBlueprint.hasItem` true _asvehicle_blueprint)
        (`SceneComponent.SetVisibility` (`self.StaticMesh`) false false)
        (set `self.Respawning` true)
        (bind _returnvalue (`KismetSystemLibrary.K2_SetTimerDelegate` (delegate `Respawn`) 5.0))
        (set `self.RespawnTimer` _returnvalue)))))

(event `Respawn`
  ;[1 1 1] Respawning
  (`SceneComponent.SetVisibility` (`self.StaticMesh`) true false)
  (set `self.Respawning` false)
  (`KismetSystemLibrary.K2_ClearAndInvalidateTimerHandle` (`self.RespawnTimer`)))

(event `self.ReceiveTick`
  (params (DeltaSeconds :type "Float (single-precision)"))
  (bind _staticmesh (`self.StaticMesh`))
  ;[1 1 1] Movement
  (`SceneComponent.K2_AddRelativeRotation` _staticmesh (* (`KismetMathLibrary.MakeRotator` 0.0 0.0 15.0) (`GameplayStatics.GetWorldDeltaSeconds`)) false false)
  (`SceneComponent.K2_SetRelativeLocation` _staticmesh (`KismetMathLibrary.MakeVector` 0.0 0.0 (+ (* (`KismetMathLibrary.DegSin` (* (`self.GetGameTimeSinceCreation`) 100.0)) 15.0) 75.0)) false false))

(fn `UserConstructionScript`)