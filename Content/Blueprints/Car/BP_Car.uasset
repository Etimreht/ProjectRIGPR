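; BP_Car is a drivable car built on physics, moved by torque on its wheels rather than a movement component.
; MoveRight sets front axle constraint swing limits and applies yaw torque to the front wheels to steer.
; MoveForward ramps a clamped EngineTorque up, down or into reverse and applies it to the rear wheels.
; Mouse wheel input zooms the camera by changing spring arm length.
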(event `InputAxis|MoveRight`
  (params (AxisValue :type "Float (single-precision)"))
  (bind _steering_torque (`self.Steering Torque`))
  (bind _axfl (`self.AXFL`))
  (bind _wheelfr (`self.WheelFR`))
  ;[1 1 1] STEERING     D= right + 1 A= left -1 None= 0
  (`/Engine/EditorBlueprintResources/StandardMacros.CompareFloat` AxisValue
    (:`>`
      (`PhysicsConstraintComponent.SetAngularSwing1Limit` _axfl "ACM_Limited" 30.0)
      (`PrimitiveComponent.AddTorqueInDegrees` _wheelfr (`KismetMathLibrary.MakeVector` 0.0 0.0 _steering_torque) "None" true)
      (`PrimitiveComponent.AddTorqueInDegrees` (`self.WheelFL`) (`KismetMathLibrary.MakeVector` 0.0 0.0 _steering_torque) "None" true))
    (:`<`
      (`PhysicsConstraintComponent.SetAngularSwing1Limit` _axfl "ACM_Limited" -30.0)
      (`PhysicsConstraintComponent.SetAngularSwing1Limit` (`self.AXFR`) "ACM_Limited" -30.0)
      (`PrimitiveComponent.AddTorqueInDegrees` _wheelfr (`KismetMathLibrary.MakeVector` 0.0 0.0 (* _steering_torque -1.0)) "None" true)
      (`PrimitiveComponent.AddTorqueInDegrees` (`self.WheelFL`) (`KismetMathLibrary.MakeVector` 0.0 0.0 (* _steering_torque -1.0)) "None" true))))

(event `InputAxis|MoveForward`
  (params (AxisValue :type "Float (single-precision)"))
  ;[1 1 1] Applies Torque to back wheels
  (`/Engine/EditorBlueprintResources/StandardMacros.CompareFloat` AxisValue
    (:`>`
      (bind _output_get (set `self.Engine Torque` (`KismetMathLibrary.FClamp` (+ (`self.Engine Torque`) 5000.0) 0.0 60000.0)))
      (`PrimitiveComponent.AddTorqueInDegrees` (`self.WheelBR`) (`KismetMathLibrary.MakeVector` 0.0 _output_get) "None" true)
      (`PrimitiveComponent.AddTorqueInDegrees` (`self.WheelBL`) (`KismetMathLibrary.MakeVector` 0.0 _output_get) "None" true))
    (:`==`
      (bind _output_get_2 (set `self.Engine Torque` (`KismetMathLibrary.FClamp` (- (`self.Engine Torque`) 10000.0) 0.0 60000.0)))
      (`PrimitiveComponent.AddTorqueInDegrees` (`self.WheelBR`) (`KismetMathLibrary.MakeVector` 0.0 _output_get_2) "None" true)
      (`PrimitiveComponent.AddTorqueInDegrees` (`self.WheelBL`) (`KismetMathLibrary.MakeVector` 0.0 _output_get_2) "None" true))
    (:`<`
      (bind _output_get_3 (set `self.Engine Torque` (`KismetMathLibrary.FClamp` (- (`self.Engine Torque`) 5000.0) -30000.0)))
      (`PrimitiveComponent.AddTorqueInDegrees` (`self.WheelBR`) (`KismetMathLibrary.MakeVector` 0.0 _output_get_3) "None" true)
      (`PrimitiveComponent.AddTorqueInDegrees` (`self.WheelBL`) (`KismetMathLibrary.MakeVector` 0.0 _output_get_3) "None" true))))

(event `Key|MouseScrollDown`
  (params (Key :type "Key Structure"))
  (bind _springarm (`self.SpringArm`))
  ;[1 1 1] Camera Zoom
  (:`Pressed`
    (set `SpringArmComponent.TargetArmLength` (+ (`SpringArmComponent.TargetArmLength` _springarm) 30.0) _springarm :!label _label))
  (:`Released`
    (goto _label)))

(event `Key|MouseScrollUp`
  (params (Key :type "Key Structure"))
  (bind _springarm (`self.SpringArm`))
  ;[1 1 1] Camera Zoom
  (:`Pressed`
    (set `SpringArmComponent.TargetArmLength` (- (`SpringArmComponent.TargetArmLength` _springarm) 30.0) _springarm :!label _label_2))
  (:`Released`
    (goto _label_2)))

(fn `UserConstructionScript`)