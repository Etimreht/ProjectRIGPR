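; Nos pickup pad that tops up an overlapping VehicleBlueprint's Nos by a fixed amount, clamped to full.
; A successful pickup hides the mesh and particles and starts a timer that restores the pad, while a full vehicle only triggers a printed message.
; A DoOnce on the pill collision, reset when a vehicle leaves, and an IsRespawning flag prevent repeat pickups.
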(event `self.PillCollision.OnComponentBeginOverlap`
  (params (OverlappedComponent :type "PrimitiveComponent Object Reference") (OtherActor :type "Actor Object Reference") (OtherComp :type "PrimitiveComponent Object Reference") (OtherBodyIndex :type Integer) (bFromSweep :type Boolean) (SweepResult :type "HitResult Structure (by ref)"))
  (`/Engine/EditorBlueprintResources/StandardMacros.DoOnce` false :!label _label
    (:`Completed`
      (if (not (`self.isRespawning`))
        (bind _asvehicle_blueprint (cast `/Game/Blueprints/PlayerVehicle/VehicleBlueprint` OtherActor))
        (if (>= (`/Game/Blueprints/PlayerVehicle/VehicleBlueprint.Nos` _asvehicle_blueprint) 1.0)
          (`KismetSystemLibrary.PrintString` "You are full on Nos!")
          (else
            (set `/Game/Blueprints/PlayerVehicle/VehicleBlueprint.Nos` (`KismetMathLibrary.FClamp` (+ (`/Game/Blueprints/PlayerVehicle/VehicleBlueprint.Nos` _asvehicle_blueprint) 0.2)) _asvehicle_blueprint)
            (`SceneComponent.SetVisibility` (`self.NosMesh`) false false)
            (`ActorComponent.SetActive` (`self.NOSParticles`) false false)
            (set `self.isRespawning` true)
            (bind _returnvalue (`KismetSystemLibrary.K2_SetTimerDelegate` (delegate `PadRespawn`) 10.0))
            (set `self.RespawnTimer` _returnvalue)))))))

(event `self.PillCollision.OnComponentEndOverlap`
  (params (OverlappedComponent :type "PrimitiveComponent Object Reference") (OtherActor :type "Actor Object Reference") (OtherComp :type "PrimitiveComponent Object Reference") (OtherBodyIndex :type Integer))
  (cast `/Game/Blueprints/PlayerVehicle/VehicleBlueprint` OtherActor)
  (goto _label :!via `Reset`))

(event `PadRespawn`
  ;[1 1 1] Nos Pad Respawn
  (`KismetSystemLibrary.PrintString` "Nos Pad Respawned!")
  (`SceneComponent.SetVisibility` (`self.NosMesh`) true false)
  (`ActorComponent.SetActive` (`self.NOSParticles`) true false)
  (set `self.isRespawning` false)
  (`KismetSystemLibrary.K2_ClearAndInvalidateTimerHandle` (`self.RespawnTimer`)))

(fn `UserConstructionScript`)