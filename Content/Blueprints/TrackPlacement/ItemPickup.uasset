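; Track item pickup that gives its item type (missile, speed boost or EMP) to an overlapping VehicleBlueprint whose item slot is empty.
; The construction script sets the matching material and icon mesh, destroys the other two, and treats None as Missile.
; Tick bobs the mesh on a sine wave and spins the icon's scene root by a fixed per-frame step.
; Collection hides the pickup and blocks reuse until a five-second timer respawns it.
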(event `self.Collider.OnComponentBeginOverlap`
  (params (OverlappedComponent :type "PrimitiveComponent Object Reference") (OtherActor :type "Actor Object Reference") (OtherComp :type "PrimitiveComponent Object Reference") (OtherBodyIndex :type Integer) (bFromSweep :type Boolean) (SweepResult :type "HitResult Structure (by ref)"))
  ;[1 1 1] Touched by a Car
  (if (not (`self.Respawning`))
    (bind _asvehicle_blueprint (cast `/Game/Blueprints/PlayerVehicle/VehicleBlueprint` OtherActor))
    (switch `/Game/Blueprints/TrackPlacement/Item_ENUM` (`/Game/Blueprints/PlayerVehicle/VehicleBlueprint.CurrentItem` _asvehicle_blueprint)
      (:`NewEnumerator0`
        (`/Game/Blueprints/PlayerVehicle/VehicleBlueprint.SetItem` _asvehicle_blueprint (`self.ItemType`))
        (`SceneComponent.SetVisibility` (`self.StaticMesh`) false true)
        (set `self.Respawning` true)
        (bind _returnvalue (`KismetSystemLibrary.K2_SetTimerDelegate` (delegate `Respawn`) 5.0))
        (set `self.RespawnTimer` _returnvalue)))))

(event `self.ReceiveTick`
  (params (DeltaSeconds :type "Float (single-precision)"))
  ;[1 1 1] Movement
  (`SceneComponent.K2_SetRelativeLocation` (`self.StaticMesh`) (`KismetMathLibrary.MakeVector` 0.0 0.0 (+ (* (`KismetMathLibrary.DegSin` (* (`self.GetGameTimeSinceCreation`) 100.0)) 15.0) 60.0)) false false)
  (`SceneComponent.K2_AddWorldRotation` (`self.Scene`) (`KismetMathLibrary.MakeRotator` 0.0 0.0 -1.0) false false))

(event `Respawn`
  ;[1 1 1] Respawning
  (`SceneComponent.SetVisibility` (`self.StaticMesh`) true true)
  (`SceneComponent.SetVisibility` (`self.Scene`) true true)
  (set `self.Respawning` false)
  (`KismetSystemLibrary.K2_ClearAndInvalidateTimerHandle` (`self.RespawnTimer`)))

(fn `UserConstructionScript`
  (`SceneComponent.SetVisibility` (`self.Scene`) false true)
  (switch `/Game/Blueprints/TrackPlacement/Item_ENUM` (`self.ItemType`) :!label _label
    (:`NewEnumerator0`
      (set `self.ItemType` "NewEnumerator1")
      (goto _label))
    (:`NewEnumerator1`
      (`PrimitiveComponent.SetMaterial` (`self.StaticMesh`) 0 "/Game/Materials/ItemPickup_Mat_Missile.ItemPickup_Mat_Missile")
      (`SceneComponent.SetVisibility` (`self.MissileMesh`) true false)
      (`ActorComponent.K2_DestroyComponent` (`self.SpeedMesh`))
      (`ActorComponent.K2_DestroyComponent` (`self.EMPMesh`)))
    (:`NewEnumerator2`
      (`PrimitiveComponent.SetMaterial` (`self.StaticMesh`) 0 "/Game/Materials/ItemPickup_Mat_Speed.ItemPickup_Mat_Speed")
      (`SceneComponent.SetVisibility` (`self.SpeedMesh`) true false)
      (`ActorComponent.K2_DestroyComponent` (`self.MissileMesh`))
      (`ActorComponent.K2_DestroyComponent` (`self.EMPMesh`)))
    (:`NewEnumerator3`
      (`PrimitiveComponent.SetMaterial` (`self.StaticMesh`) 0 "/Game/Materials/ItemPickup_Mat_Emp.ItemPickup_Mat_Emp")
      (`SceneComponent.SetVisibility` (`self.EMPMesh`) true false)
      (`ActorComponent.K2_DestroyComponent` (`self.MissileMesh`))
      (`ActorComponent.K2_DestroyComponent` (`self.SpeedMesh`)))))