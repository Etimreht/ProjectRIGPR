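; Race-end pawn that offers the server a return to the lobby once every car has finished.
; It gathers all VehicleBlueprint actors at BeginPlay, and on authority Tick polls their RaceFinished flags until all are done, then reveals ReturnToLobby once.
; The authority's K key then calls ResetLobby on RacerGameMode.
; A FadeIn event uses a timeline to drive the opacity of an unlit black material on an inverted sphere.
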(event `self.ReceiveBeginPlay`
  (bind _outactors (`GameplayStatics.GetAllActorsOfClass` "/Game/Blueprints/PlayerVehicle/VehicleBlueprint.VehicleBlueprint_C"))
  (set `self.AllCars` _outactors))

(event `FadeIn`
  (bind (_direction _newtrack_0) (`Timeline|Timeline_0` :!via `PlayFromStart`)
    (:`Update`
      (bind _returnvalue (`PrimitiveComponent.CreateDynamicMaterialInstance` (`self.InvertedSphere`) 0 "/Game/Materials/UnlitBlack.UnlitBlack" "None"))
      (`MaterialInstanceDynamic.SetScalarParameterValue` _returnvalue "Opacity" _newtrack_0))))

(event `Key|K`
  (params (Key :type "Key Structure"))
  (:`Pressed`
    (`/Engine/EditorBlueprintResources/ActorMacros.Switch Has Authority`
      (:`Authority`
        (if (`self.AllPlayersFinished`)
          (bind _asracer_game_mode (cast `/Game/GameData/RacerGameMode` (`GameplayStatics.GetGameMode`)))
          (`/Game/GameData/RacerGameMode.ResetLobby` _asracer_game_mode))))))

(event `self.ReceiveTick`
  (params (DeltaSeconds :type "Float (single-precision)"))
  (`/Engine/EditorBlueprintResources/ActorMacros.Switch Has Authority`
    (:`Authority`
      (if (`self.AllPlayersFinished`)
        (`/Engine/EditorBlueprintResources/StandardMacros.DoOnce` false
          (:`Completed`
            (set `self.AllPlayersFinished` true)
            (`SceneComponent.SetVisibility` (`self.ReturnToLobby`) true false)))
        (else
          (`self.CheckAllFinished`))))))

(fn `CheckAllFinished`
  (locals (AtLeastOneUnfinished :type Boolean))
  (for _array_element (`self.AllCars`)
    (if (not (`/Game/Blueprints/PlayerVehicle/VehicleBlueprint.RaceFinished` _array_element))
      (set `local.AtLeastOneUnfinished` true)))
  (if (not (`local.AtLeastOneUnfinished`))
    (set `self.AllPlayersFinished` true)))

(fn `UserConstructionScript`)