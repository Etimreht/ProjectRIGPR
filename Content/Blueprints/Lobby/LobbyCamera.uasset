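; LobbyCamera is the player's VR-capable lobby view for a racing game, handling car customization, readiness and match start.
; On begin play it recenters the headset and runs a timeline fade through a dynamic black material on a mesh.
; Tick keeps a text label floating above the lobby car.
; Input recenters VR, cycles car materials with a wrapping index, toggles plinth readiness, and lets the authority start RacerGameMode once the lobby is ready.
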(event `self.ReceiveBeginPlay`
  (`HeadMountedDisplayFunctionLibrary.ResetOrientationAndPosition` 0.0)
  (bind (_direction _opacity) (`Timeline|CameraFade` :!via `PlayFromStart`)
    (:`Update`
      (bind _returnvalue (`PrimitiveComponent.CreateDynamicMaterialInstance` (`self.StaticMesh`) 0 "/Game/Materials/UnlitBlack.UnlitBlack" "None"))
      (`MaterialInstanceDynamic.SetScalarParameterValue` _returnvalue "Opacity" _opacity))))

(event `self.ReceiveTick`
  (params (DeltaSeconds :type "Float (single-precision)"))
  (`self.TextEvent`))

(event `TextEvent`
  (bind _lobbycar (`self.LobbyCar`))
  (bind (_returnvalue_x _returnvalue_y _returnvalue_z) (`KismetMathLibrary.BreakVector` (`self.K2_GetActorLocation` _lobbycar)))
  (`/Engine/EditorBlueprintResources/StandardMacros.IsValid` _lobbycar
    (:`Is Valid`
      (`SceneComponent.K2_SetWorldLocation` (`self.TextRender`) (`KismetMathLibrary.MakeVector` _returnvalue_x _returnvalue_y (+ _returnvalue_z 100.0)) false false))))

(event `InputAction|ResetVR`
  (params (Key :type "Key Structure"))
  (:`Pressed`
    (`HeadMountedDisplayFunctionLibrary.ResetOrientationAndPosition` 0.0 :!label _label)))

(event `ResetVR`
  (goto _label))

(event `Key|K`
  (params (Key :type "Key Structure"))
  (:`Pressed`
    (`/Engine/EditorBlueprintResources/ActorMacros.Switch Has Authority`
      (:`Authority`
        (if (`/Game/Blueprints/Lobby/LobbyArea.GameReadyToStart` (`self.LobbyArea`))
          (bind _asracer_game_mode (cast `/Game/GameData/RacerGameMode` (`GameplayStatics.GetGameMode`)))
          (`/Game/GameData/RacerGameMode.StartGame` _asracer_game_mode))))))

(event `Key|Q`
  (params (Key :type "Key Structure"))
  (:`Pressed`
    (`/Game/Blueprints/PlayerVehicle/VehicleBlueprint.ChangeMaterial` (`self.LobbyCar`) -1)
    (`self.ChangeMaterialIndex` -1)))

(event `SetReady`
  (`/Game/Blueprints/Lobby/CarPlinth.SetReadyState` (`self.LobbyPlinth`) (not (`/Game/Blueprints/Lobby/CarPlinth.Ready` (`self.LobbyPlinth`)))))

(event `Key|E`
  (params (Key :type "Key Structure"))
  (:`Pressed`
    (`/Game/Blueprints/PlayerVehicle/VehicleBlueprint.ChangeMaterial` (`self.LobbyCar`) 1)
    (`self.ChangeMaterialIndex` 1)))

(event `Key|R`
  (params (Key :type "Key Structure"))
  (:`Pressed`
    (`self.SetReady`)))

(event `ChangeMaterialIndex`
  (params (NewInt :type Integer))
  (bind _returnvalue (+ NewInt (`self.MaterialIndex`)))
  (if (< _returnvalue 0)
    (set `self.MaterialIndex` 3)
    (elif (> _returnvalue 3)
      (set `self.MaterialIndex` 0)
      (else
        (set `self.MaterialIndex` _returnvalue)))))

(fn `UserConstructionScript`)