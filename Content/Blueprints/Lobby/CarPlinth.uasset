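; Lobby car plinth Blueprint whose indicator light shows the ready state of the car it references.
; Initialise sets the light to not ready when CarReference is valid and resets it to off otherwise.
; SetReadyState and Reset update the Ready flag and pass a green, red or off material to SetReadyMaterialForAll, which applies it to the ReadyLight component.
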(event `Initialise`
  (`/Engine/EditorBlueprintResources/StandardMacros.IsValid` (`self.CarReference`)
    (:`Is Valid`
      (`self.SetReadyState` false))
    (:`Is Not Valid`
      (`self.Reset`))))

(event `SetReadyState`
  (params (Ready :type Boolean))
  (bind _output_get (set `self.Ready` Ready))
  (if _output_get
    (`self.SetReadyMaterialForAll` "/Game/Materials/GreenLight.GreenLight")
    (else
      (`self.SetReadyMaterialForAll` "/Game/Materials/RedLight.RedLight"))))

(event `Reset`
  (set `self.Ready` false)
  (`self.SetReadyMaterialForAll` "/Game/Materials/OffLight.OffLight"))

(event `SetReadyMaterialForAll`
  (params (Material :type "MaterialInstance Object Reference"))
  (`PrimitiveComponent.SetMaterial` (`self.ReadyLight`) 0 Material))

(fn `UserConstructionScript`)