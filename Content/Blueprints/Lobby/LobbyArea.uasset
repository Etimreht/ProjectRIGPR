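; Lobby area actor that hosts car plinths and signals when the game is ready to start.
; On BeginPlay, the authority spawns four CarPlinth actors at scene component transforms and stores them in Plinths.
; Every Tick, ReadyCheck looks for any plinth with a valid car that is not Ready, ignoring those without cars.
; The result sets GameReadyToStart and toggles the text render's visibility.
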(event `self.ReceiveBeginPlay`
  (`/Engine/EditorBlueprintResources/ActorMacros.Switch Has Authority`
    (:`Authority`
      (bind _returnvalue (`|SpawnActorFromClass` "/Game/Blueprints/Lobby/CarPlinth.CarPlinth_C" (`SceneComponent.K2_GetComponentToWorld` (`self.Scene1`)) "Undefined" "OverrideRootScale" null null))
      (`KismetArrayLibrary.Array_Add` (`self.Plinths`) _returnvalue)
      (bind _returnvalue_2 (`|SpawnActorFromClass` "/Game/Blueprints/Lobby/CarPlinth.CarPlinth_C" (`SceneComponent.K2_GetComponentToWorld` (`self.Scene2`)) "Undefined" "OverrideRootScale" null null))
      (`KismetArrayLibrary.Array_Add` (`self.Plinths`) _returnvalue_2)
      (bind _returnvalue_3 (`|SpawnActorFromClass` "/Game/Blueprints/Lobby/CarPlinth.CarPlinth_C" (`SceneComponent.K2_GetComponentToWorld` (`self.Scene3`)) "Undefined" "OverrideRootScale" null null))
      (`KismetArrayLibrary.Array_Add` (`self.Plinths`) _returnvalue_3)
      (bind _returnvalue_4 (`|SpawnActorFromClass` "/Game/Blueprints/Lobby/CarPlinth.CarPlinth_C" (`SceneComponent.K2_GetComponentToWorld` (`self.Scene4`)) "Undefined" "OverrideRootScale" null null))
      (`KismetArrayLibrary.Array_Add` (`self.Plinths`) _returnvalue_4))))

(event `self.ReceiveTick`
  (params (DeltaSeconds :type "Float (single-precision)"))
  (`self.ReadyCheck`))

(fn `ReadyCheck`
  (locals (GameCanStart :type Boolean :default true))
  (for _array_element (`self.Plinths`)
    (if (and (`KismetSystemLibrary.IsValid` (`/Game/Blueprints/Lobby/CarPlinth.CarReference` _array_element)) (not (`/Game/Blueprints/Lobby/CarPlinth.Ready` _array_element)))
      (set `local.GameCanStart` false)
      (break)))
  (bind _output_get (set `self.GameReadyToStart` (`local.GameCanStart`)))
  (`SceneComponent.SetVisibility` (`self.TextRender`) _output_get false))

(fn `UserConstructionScript`)