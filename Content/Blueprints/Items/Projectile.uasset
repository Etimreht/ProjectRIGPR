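; Projectile is an item actor that acts as a missile, able to home in on a target and hit vehicles.
; A HomingMissile event sets a valid target as the projectile movement component's homing target.
; Overlap with a VehicleBlueprint triggers Impact, which on the authority spawns an emitter, prints a debug string, calls HitByMissile on the vehicle and destroys the projectile.
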(event `self.Projectile.OnComponentBeginOverlap`
  (params (OverlappedComponent :type "PrimitiveComponent Object Reference") (OtherActor :type "Actor Object Reference") (OtherComp :type "PrimitiveComponent Object Reference") (OtherBodyIndex :type Integer) (bFromSweep :type Boolean) (SweepResult :type "HitResult Structure (by ref)"))
  (bind (_asvehicle_blueprint _bsuccess) (cast `/Game/Blueprints/PlayerVehicle/VehicleBlueprint` OtherActor :!pure true))
  (if _bsuccess
    (`self.Impact` _asvehicle_blueprint)))

(event `HomingMissile`
  (params (Target :type "StaticMeshComponent Object Reference"))
  (`/Engine/EditorBlueprintResources/StandardMacros.IsValid` Target
    (:`Is Valid`
      (set `ProjectileMovementComponent.HomingTargetComponent` Target (`self.ProjectileMovement`)))))

(event `Impact`
  (params (Vehicle :type "/Game/Blueprints/PlayerVehicle/VehicleBlueprint Object Reference"))
  (`/Engine/EditorBlueprintResources/ActorMacros.Switch Has Authority`
    (:`Authority`
      (`GameplayStatics.SpawnEmitterAtLocation` null (`self.K2_GetActorLocation`))
      (`KismetSystemLibrary.PrintString` "Hello")
      (`/Game/Blueprints/PlayerVehicle/VehicleBlueprint.HitByMissile` Vehicle)
      (`self.K2_DestroyActor`))))

(fn `UserConstructionScript`)