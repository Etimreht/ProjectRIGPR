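; Spline-driven race course builder that generates track, verge and guard rail meshes in the construction script.
; It resizes CourseDataArray to match the spline point count, then calls BuildRaceCourse for each piece enabled on every segment, wrapping when TrackLoop is set.
; BuildRaceCourse adds spline mesh components with per-point bank and width and optional collision.
; An optional debug pass adds numbered text labels at each spline point.
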(fn `BuildRaceCourse`
  (params (CurrentLoopIndex :type Integer) (TrackRoadMesh :type "StaticMesh Object Reference"))
  (locals (Local_Current_Loop_Index :type Integer) (Local_Current_Next_Index :type Integer) (Local_Track_Road_Mesh :type "StaticMesh Object Reference" :default "StaticMesh'/Game/Geometry/StaticMeshes/Environment/Road/Track.Track'") (Local_StartLocation :type "Vector Structure") (Local_StartTangent :type "Vector Structure") (Local_EndLocation :type "Vector Structure") (Local_EndTangent :type "Vector Structure") (Local_Current_Spline_Mesh :type "SplineMeshComponent Object Reference") (Local_StartWidth :type "Float (double-precision)") (Local_StartRoll :type "Float (double-precision)") (Local_EndRoll :type "Float (double-precision)") (Local_EndWidth :type "Float (double-precision)"))
  (bind (_location _tangent) (`SplineComponent.GetLocationAndTangentAtSplinePoint` (`self.Spline`) (`local.Local_Current_Next_Index`) "Local"))
  (bind (_location_2 _tangent_2) (`SplineComponent.GetLocationAndTangentAtSplinePoint` (`self.Spline`) (`local.Local_Current_Loop_Index`) "Local"))
  (bind (_output_left_verge _output_left_guard_rail _output_rightverge _output_right_guard_rail _output_track _output_track_bank _output_track_width) (break `/Game/Blueprints/Environment/CourseData` (`|GetArrayItem` (`self.CourseDataArray`) (`local.Local_Current_Next_Index`))))
  (bind (_output_left_verge_2 _output_left_guard_rail_2 _output_rightverge_2 _output_right_guard_rail_2 _output_track_2 _output_track_bank_2 _output_track_width_2) (break `/Game/Blueprints/Environment/CourseData` (`|GetArrayItem` (`self.CourseDataArray`) (`local.Local_Current_Loop_Index`))))
  (set `local.Local_Current_Loop_Index` CurrentLoopIndex)
  (set `local.Local_Current_Next_Index` (mod (+ CurrentLoopIndex 1) (`self.Spline Points`)))
  (set `local.Local_Track_Road_Mesh` TrackRoadMesh)
  (`|ExecutionSequence`
    (:`then_0`
      (set `local.Local_StartLocation` _location_2)
      (set `local.Local_StartTangent` _tangent_2)
      (set `local.Local_EndLocation` _location)
      (set `local.Local_EndTangent` _tangent)
      (set `local.Local_StartRoll` _output_track_bank_2)
      (set `local.Local_StartWidth` _output_track_width_2)
      (set `local.Local_EndRoll` _output_track_bank)
      (set `local.Local_EndWidth` _output_track_width))
    (:`then_1`
      (bind _returnvalue (`AddComponent|NODE_AddSplineMeshComponent-2`))
      (set `local.Local_Current_Spline_Mesh` _returnvalue)
      (`StaticMeshComponent.SetStaticMesh` (`local.Local_Current_Spline_Mesh`) (`local.Local_Track_Road_Mesh`))
      (`SplineMeshComponent.SetStartAndEnd` (`local.Local_Current_Spline_Mesh`) (`local.Local_StartLocation`) (`local.Local_StartTangent`) (`local.Local_EndLocation`) (`local.Local_EndTangent`) true)
      (`SplineMeshComponent.SetStartRoll` (`local.Local_Current_Spline_Mesh`) (`local.Local_StartRoll`) true)
      (`SplineMeshComponent.SetEndRoll` (`local.Local_Current_Spline_Mesh`) (`local.Local_EndRoll`) true)
      (`SplineMeshComponent.SetStartScale` (`local.Local_Current_Spline_Mesh`) (`KismetMathLibrary.MakeVector2D` (`local.Local_StartWidth`) 1.0) true)
      (`SplineMeshComponent.SetEndScale` (`local.Local_Current_Spline_Mesh`) (`KismetMathLibrary.MakeVector2D` (`local.Local_EndWidth`) 1.0) true)
      (`PrimitiveComponent.SetCollisionEnabled` (`local.Local_Current_Spline_Mesh`) (select `bool` (`self.Collisions`) :`false` "NoCollision" :`true` "QueryAndPhysics" :!type "ECollisionEnabled Enum")))))

(fn `UserConstructionScript`
  (locals (Course_Data_Default :type "/Game/Blueprints/Environment/CourseData Structure" :default (struct :`Left_Verge` true :`Left_Guard_Rail` true :`RightVerge` true :`Right_Guard_Rail` true :`Track` true :`Track_Width` 1.0 :`Left_Verge_Width` 1.0 :`Right_Verge_Width` 1.0)) (NewLocalVar_0 :type Text))
  (bind (_output_left_verge _output_left_guard_rail _output_rightverge _output_right_guard_rail _output_track) (break `/Game/Blueprints/Environment/CourseData` (`|GetArrayItem` (`self.CourseDataArray`) (`self.CurrentLoopIndex`))))
  (`|ExecutionSequence`
    (:`then_0`
      ;[0.02263 0.194 0.1979] Store Spline Points to variable
      (set `self.Spline Points` (`SplineComponent.GetNumberOfSplinePoints` (`self.Spline`))))
    (:`then_1`
      ;[1 1 1] Comment
      (`/Engine/EditorBlueprintResources/StandardMacros.CompareInt` (`KismetArrayLibrary.Array_Length` (`self.CourseDataArray`)) (`self.Spline Points`) :!label _label
        (:`>`
          (`KismetArrayLibrary.Array_Remove` (`self.CourseDataArray`))
          (goto _label))
        (:`<`
          (`KismetArrayLibrary.Array_Add` (`self.CourseDataArray`) (`local.Course_Data_Default`))
          (goto _label))))
    (:`then_2`
      (for _index (range (+ (- (`self.Spline Points`) (`KismetMathLibrary.SelectInt` 1 2 (`self.Track Loop?`))) 1))
        (set `self.CurrentLoopIndex` _index)
        (set `self.Draw_Left_Guard_Rail` _output_left_guard_rail)
        (set `self.Draw_Right_Guard_Rail` _output_right_guard_rail)
        (set `self.Draw_Left_Verge` _output_left_verge)
        (set `self.Draw_Right_Verge` _output_rightverge)
        (set `self.Draw_Track` _output_track)
        (`|ExecutionSequence`
          (:`then_0`
            (if (`self.Draw_Track`)
              (`self.BuildRaceCourse` (`self.CurrentLoopIndex`) (`self.Track`))))
          (:`then_1`
            (if (`self.Draw_Left_Verge`)
              (`self.BuildRaceCourse` (`self.CurrentLoopIndex`) (`self.Left_Verge`))))
          (:`then_2`
            (if (`self.Draw_Right_Verge`)
              (`self.BuildRaceCourse` (`self.CurrentLoopIndex`) (`self.Right_Verge`))))
          (:`then_3`
            (if (`self.Draw_Left_Guard_Rail`)
              (`self.BuildRaceCourse` (`self.CurrentLoopIndex`) (`self.Left_Guard_Rail`))))
          (:`then_4`
            (if (`self.Draw_Right_Guard_Rail`)
              (`self.BuildRaceCourse` (`self.CurrentLoopIndex`) (`self.Right_Guard_Rail`)))))))
    (:`then_3`
      (if (`self.Draw Track Point Numbers`)
        (for _index_2 (range (`self.Spline Points`))
          (set `self.Current Track Point` (`KismetStringLibrary.Conv_IntToString` _index_2))
          (bind (_location _tangent) (`SplineComponent.GetLocationAndTangentAtSplinePoint` (`self.Spline`) _index_2 "Local"))
          (bind _returnvalue (`AddComponent|NODE_AddTextRenderComponent-0` :`RelativeTransform` (`KismetMathLibrary.MakeTransform` (`KismetMathLibrary.MakeVector` (.x _location) (.y _location) (+ (.z _location) 25.0)) (`KismetMathLibrary.Conv_VectorToRotator` (* _tangent -1.0)))))
          (`TextRenderComponent.K2_SetText` _returnvalue (`KismetTextLibrary.Conv_StringToText` (`self.Current Track Point`))))))))