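; Spline actor Blueprint that lays a chosen static mesh along its spline, deforming it to follow the curve.
; The construction script adds a spline mesh component for each point index, using that point and the next for local-space positions, tangents and scales.
; Forward axis comes from a variable, roll is fixed at zero, and collision is query-only.
; The event graph holds only disabled placeholder events.
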(fn `UserConstructionScript`
  (bind _spline (`self.Spline`))
  (for _index (range (`SplineComponent.GetNumberOfSplinePoints` _spline))
    (bind _returnvalue (`AddComponent|NODE_AddSplineMeshComponent-0`))
    (`StaticMeshComponent.SetStaticMesh` _returnvalue (`self.Static Mesh`))
    (`SplineMeshComponent.SetForwardAxis` _returnvalue (`self.NewVar_0`) true)
    (`SceneComponent.K2_AttachToComponent` _returnvalue _spline "None" "KeepRelative" "KeepRelative" "KeepRelative" true)
    (bind _returnvalue_2 (+ _index 1))
    (`SplineMeshComponent.SetStartAndEnd` _returnvalue (`SplineComponent.GetLocationAtSplinePoint` _spline _index "Local") (`SplineComponent.GetTangentAtSplinePoint` _spline _index "Local") (`SplineComponent.GetLocationAtSplinePoint` _spline _returnvalue_2 "Local") (`SplineComponent.GetTangentAtSplinePoint` _spline _returnvalue_2 "Local") true)
    (`SplineMeshComponent.SetStartScale` _returnvalue (`KismetMathLibrary.Conv_VectorToVector2D` (`SplineComponent.GetScaleAtSplinePoint` _spline _index)) true)
    (`SplineMeshComponent.SetEndScale` _returnvalue (`KismetMathLibrary.Conv_VectorToVector2D` (`SplineComponent.GetScaleAtSplinePoint` _spline (+ 1 _index))) true)
    (`SplineMeshComponent.SetStartRoll` _returnvalue 0.0 true)
    (`SplineMeshComponent.SetEndRoll` _returnvalue 0.0 true)
    (`PrimitiveComponent.SetCollisionEnabled` _returnvalue "QueryOnly")))