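; Race checkpoint actor that tracks vehicle progress and doubles as the finish line when IsFinishLine is set.
; A DoOnce-guarded overlap accepts checkpoints only in numbered order, storing the latest on the VehicleBlueprint.
; The finish line requires the last checkpoint, then records a lap time or ends the race on lap three.
; It also shows timed start lights with pips, and the authority notifies the GameMode when the countdown completes.
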(event `IsCheckpoint`
  (params (`Other Actor` :type "/Game/VehicleAdvBP/Blueprints/VehicleBlueprint Object Reference"))
  (set `/Game/VehicleAdvBP/Blueprints/VehicleBlueprint.CurrentCheckPoint` self `Other Actor`)
  (`KismetSystemLibrary.PrintString` (`KismetStringLibrary.Conv_IntToString` (`self.CheckPointNo`)))
  (`KismetSystemLibrary.PrintString` (`KismetStringLibrary.Conv_VectorToString` (`SceneComponent.K2_GetComponentLocation` (`self.DefaultSceneRoot`)))))

(event `NewLap`
  (params (`Other Actor` :type "/Game/VehicleAdvBP/Blueprints/VehicleBlueprint Object Reference"))
  (bind _laptime (`/Game/VehicleAdvBP/Blueprints/VehicleBlueprint.LapTime` `Other Actor`))
  (set `/Game/VehicleAdvBP/Blueprints/VehicleBlueprint.CurrentCheckPoint` self `Other Actor`)
  (bind _output_get (set `/Game/VehicleAdvBP/Blueprints/VehicleBlueprint.LapNumber` (`KismetMathLibrary.Clamp` (+ (`/Game/VehicleAdvBP/Blueprints/VehicleBlueprint.LapNumber` `Other Actor`) 1) 0 3) `Other Actor`))
  (`KismetSystemLibrary.PrintString` (`KismetStringLibrary.Conv_IntToString` _output_get))
  (`KismetArrayLibrary.Array_Add` (`/Game/VehicleAdvBP/Blueprints/VehicleBlueprint.LapTimes` `Other Actor`) _laptime)
  (`KismetSystemLibrary.PrintString` (`KismetStringLibrary.Conv_DoubleToString` _laptime))
  (set `/Game/VehicleAdvBP/Blueprints/VehicleBlueprint.LapTime` 0.0 `Other Actor`))

(event `FinishLine`
  (params (`Other Actor` :type "/Game/VehicleAdvBP/Blueprints/VehicleBlueprint Object Reference"))
  (set `/Game/VehicleAdvBP/Blueprints/VehicleBlueprint.CurrentCheckPoint` self `Other Actor`)
  (`/Game/VehicleAdvBP/Blueprints/VehicleBlueprint.FinishGame` `Other Actor`)
  (`self.DisableInput` `Other Actor` (`GameplayStatics.GetPlayerController` 0))
  (`KismetSystemLibrary.PrintString` "Race Finished")
  (for _array_element (`/Game/VehicleAdvBP/Blueprints/VehicleBlueprint.LapTimes` `Other Actor`)
    (`KismetSystemLibrary.PrintString` (`KismetStringLibrary.Conv_IntToString` (`KismetMathLibrary.Round` _array_element))))
  (`KismetSystemLibrary.PrintString` (`KismetStringLibrary.Concat_StrStr` "Total Time: " (`KismetStringLibrary.Conv_DoubleToString` (`/Game/VehicleAdvBP/Blueprints/VehicleBlueprint.RaceTime` `Other Actor`)))))

(event `self.Checkpoint.OnComponentBeginOverlap`
  (params (OverlappedComponent :type "PrimitiveComponent Object Reference") (OtherActor :type "Actor Object Reference") (OtherComp :type "PrimitiveComponent Object Reference") (OtherBodyIndex :type Integer) (bFromSweep :type Boolean) (SweepResult :type "HitResult Structure (by ref)"))
  (bind _asvehicle_blueprint (cast `/Game/VehicleAdvBP/Blueprints/VehicleBlueprint` OtherActor))
  (`/Engine/EditorBlueprintResources/StandardMacros.DoOnce` false :!label _label
    (:`Completed`
      (if (`self.isFinishLine`)
        (if (`self.CanCrossFinishLine` _asvehicle_blueprint)
          (if (>= (`/Game/VehicleAdvBP/Blueprints/VehicleBlueprint.LapNumber` (cast `/Game/VehicleAdvBP/Blueprints/VehicleBlueprint` OtherActor :!pure true)) 3)
            (`self.FinishLine` _asvehicle_blueprint)
            (else
              (`self.NewLap` _asvehicle_blueprint))))
        (elif (== (`/Game/Geometry/Blueprint/CheckPoint.CheckPointNo` (`/Game/VehicleAdvBP/Blueprints/VehicleBlueprint.CurrentCheckPoint` _asvehicle_blueprint)) (- (`self.CheckPointNo`) 1))
          (`self.ischeckpoint` _asvehicle_blueprint))))))

(event `self.Checkpoint.OnComponentEndOverlap`
  (params (OverlappedComponent :type "PrimitiveComponent Object Reference") (OtherActor :type "Actor Object Reference") (OtherComp :type "PrimitiveComponent Object Reference") (OtherBodyIndex :type Integer))
  (goto _label :!via `Reset`))

(event `CountdownLightsEvent`
  (params (GameMode :type "/Game/GameData/RacerGameMode Object Reference"))
  (`PrimitiveComponent.SetMaterial` (`self.Light1`) 0 "/Game/Materials/OffLight.OffLight")
  (`PrimitiveComponent.SetMaterial` (`self.Light2`) 0 "/Game/Materials/OffLight.OffLight")
  (`PrimitiveComponent.SetMaterial` (`self.Light3`) 0 "/Game/Materials/OffLight.OffLight")
  ;[1 0.06103 0] 3
  (`KismetSystemLibrary.Delay` 3.0)
  (`PrimitiveComponent.SetMaterial` (`self.Light1`) 0 "/Game/Materials/RedLight.RedLight")
  (`GameplayStatics.PlaySoundAtLocation` "/Game/SFX/CountdownPip.CountdownPip" (`SceneComponent.K2_GetComponentLocation` (`self.CountdownLights`)) (struct) 1.0 1.0 0.0 null null null)
  ;[1 0.06103 0] 2
  (`KismetSystemLibrary.Delay` 1.0)
  (`PrimitiveComponent.SetMaterial` (`self.Light2`) 0 "/Game/Materials/RedLight.RedLight")
  (`GameplayStatics.PlaySoundAtLocation` "/Game/SFX/CountdownPip.CountdownPip" (`SceneComponent.K2_GetComponentLocation` (`self.CountdownLights`)) (struct) 1.0 1.0 0.0 null null null)
  ;[1 0.06103 0] 1
  (`KismetSystemLibrary.Delay` 1.0)
  (`PrimitiveComponent.SetMaterial` (`self.Light3`) 0 "/Game/Materials/RedLight.RedLight")
  (`GameplayStatics.PlaySoundAtLocation` "/Game/SFX/CountdownPip.CountdownPip" (`SceneComponent.K2_GetComponentLocation` (`self.CountdownLights`)) (struct) 1.0 1.0 0.0 null null null)
  ;[0.0122 1 0] Go!
  (`KismetSystemLibrary.Delay` 1.0)
  (`PrimitiveComponent.SetMaterial` (`self.Light3`) 0 "/Game/Materials/GreenLight.GreenLight")
  (`PrimitiveComponent.SetMaterial` (`self.Light1`) 0 "/Game/Materials/GreenLight.GreenLight")
  (`PrimitiveComponent.SetMaterial` (`self.Light2`) 0 "/Game/Materials/GreenLight.GreenLight")
  (`GameplayStatics.PlaySoundAtLocation` "/Game/SFX/CountdownPip2.CountdownPip2" (`SceneComponent.K2_GetComponentLocation` (`self.CountdownLights`)) (struct) 1.3 2.5 0.0 null null null)
  (`/Engine/EditorBlueprintResources/ActorMacros.Switch Has Authority`
    (:`Authority`
      (`/Game/GameData/RacerGameMode.CountdownComplete` GameMode))))

(fn `CanCrossFinishLine`
  (params (Player :type "/Game/VehicleAdvBP/Blueprints/VehicleBlueprint Object Reference"))
  (returns (True :type Boolean))
  (return (== (`/Game/Geometry/Blueprint/CheckPoint.CheckPointNo` (`/Game/VehicleAdvBP/Blueprints/VehicleBlueprint.CurrentCheckPoint` Player)) (- (`KismetArrayLibrary.Array_Length` (`/Game/VehicleAdvBP/Blueprints/VehicleBlueprint.AllCheckpoints` Player)) 1))))

(fn `UserConstructionScript`
  (if (`self.isFinishLine`)
    (`SceneComponent.SetVisibility` (`self.Text`) false false)
    (else
      (`SceneComponent.SetVisibility` (`self.CountdownLights`) false true))))